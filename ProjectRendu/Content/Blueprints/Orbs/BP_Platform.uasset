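; BP_Platform is a pickup platform that spawns a BP_Orbs actor just above itself and respawns it after it is taken.
; Any overlap with its Box destroys the orb and clears HaveOrbs, and an overlapping BP_ThirdPersonCharacter gets its HaveOrb flag set.
; Tick polls HaveOrbs and, while it is false, runs a five-second Delay into the same spawn logic BeginPlay uses.
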(event `self.ReceiveBeginPlay`
  (if (not (`self.HaveOrbs`))
    (bind _returnvalue (`|SpawnActorFromClass` "/Game/Blueprints/Orbs/BP_Orbs.BP_Orbs_C" (`KismetMathLibrary.MakeTransform` (+ (`self.K2_GetActorLocation`) (0.0 0.0 50.0))) "Undefined" "MultiplyWithRoot" null null :!label _label))
    (set `self.HaveOrbs` true)))

(event `self.ReceiveTick`
  (params (DeltaSeconds :type "Float (single-precision)"))
  (if (== (`self.HaveOrbs`) false)
    (`KismetSystemLibrary.Delay` 5.0)
    (goto _label)))

(event `self.Box.OnComponentBeginOverlap`
  (params (OverlappedComponent :type "PrimitiveComponent Object Reference") (OtherActor :type "Actor Object Reference") (OtherComp :type "PrimitiveComponent Object Reference") (OtherBodyIndex :type Integer) (bFromSweep :type Boolean) (SweepResult :type "HitResult Structure (by ref)"))
  (`self.K2_DestroyActor` (stale `self.ReceiveBeginPlay` _returnvalue))
  (set `self.HaveOrbs` false)
  (bind _asbp_third_person_character (cast `/Game/ThirdPerson/Blueprints/BP_ThirdPersonCharacter` OtherActor))
  (set `/Game/ThirdPerson/Blueprints/BP_ThirdPersonCharacter.HaveOrb` true _asbp_third_person_character))

(fn `UserConstructionScript`)